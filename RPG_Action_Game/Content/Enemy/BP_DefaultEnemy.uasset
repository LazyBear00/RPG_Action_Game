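; Base-style enemy Blueprint with a capsule and a world-space health bar widget.
; On BeginPlay it registers itself as the owner of its UI_EnemyHealthBar widget.
; Every tick it rotates the health bar to face the player camera.
; A disconnected branch, noted as not working, would make the capsule ignore the Pawn channel when dead.
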(event EventBeginPlay
  (bind _asui_enemy_health_bar (Utilities|Casting|CastToUI_EnemyHealthBar (UserInterface|GetUserWidgetObject (Variables|Default|GetHealthBar))))
  (Variables|/Game/Enemy/UI_EnemyHealthBar.UI_EnemyHealthBar_C|SetHealthBarOwner _asui_enemy_health_bar self))

(event EventTick
  (params (DeltaSeconds :type Float%20%28single-precision%29))
  (bind _healthbar (Variables|Default|GetHealthBar))
  (Transformation|SetWorldRotation _healthbar (Math|Rotator|FindLookatRotation (Transformation|GetWorldLocation _healthbar) (Transformation|GetWorldLocation (Variables|/Script/Engine.PlayerCameraManager|GetTransformComponent (Game|GetPlayerCameraManager 0)))) false false))

(fn ConstructionScript)