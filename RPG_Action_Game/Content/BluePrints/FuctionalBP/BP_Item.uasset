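; BP_Item is an item actor that shows an equip prompt while the player character overlaps it.
; Overlap begin sets IsOverlappingItem on RPG_Action_GameCharacter, creates UI_EquipItemPrompt, passes it to SetCorrectItemName and adds it to the viewport.
; Overlap end clears the flag and removes all top-level prompt widgets of that class.
; SetCorrectItemName is empty here, leaving the prompt's item name unset.
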(event Collision|EventActorBeginOverlap
  (params (OtherActor :type Actor%20Object%20Reference))
  (bind _asrpg_action_game_character (Utilities|Casting|CastToRPG_Action_GameCharacter OtherActor))
  (Variables|/Script/RPG_Action_Game.RPG_Action_GameCharacter|SetisOverlappingItem _asrpg_action_game_character true)
  (bind _returnvalue (UserInterface|CreateWidget "/Game/BluePrints/FuctionalBP/UI_EquipItemPrompt.UI_EquipItemPrompt_C"))
  (CallFunction|SetCorrectItemName _returnvalue)
  (UserInterface|Viewport|AddtoViewport _returnvalue 0))

(event Collision|EventActorEndOverlap
  (params (OtherActor :type Actor%20Object%20Reference))
  (bind _asrpg_action_game_character (Utilities|Casting|CastToRPG_Action_GameCharacter OtherActor))
  (Variables|/Script/RPG_Action_Game.RPG_Action_GameCharacter|SetisOverlappingItem _asrpg_action_game_character false)
  (bind _foundwidgets (Widget|GetAllWidgetsOfClass "/Game/BluePrints/FuctionalBP/UI_EquipItemPrompt.UI_EquipItemPrompt_C" true))
  (for _array_element _foundwidgets
    (Widget|RemovefromParent _array_element)))

(fn ConstructionScript)

(fn SetCorrectItemName
  (params (NewParam :type UI%20Equip%20Item%20Prompt%20Object%20Reference)))